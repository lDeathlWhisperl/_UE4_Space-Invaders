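; BP_DeathStar is a Death Star map component that plays a purely visual superlaser firing effect at random intervals.
; Each Tick has a small random chance to start the Shot timeline, with a Wait flag blocking overlapping shots.
; The timeline's float is truncated to an index that reveals the eight lasers, then the Center beam appears after a delay.
; All parts hide after a hold, and the flag clears.
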(event `self.ReceiveBeginPlay`
  (set `self.Lasers` (`|MakeArray` (`self.Laser1`) (`self.Laser2`) (`self.Laser3`) (`self.Laser4`) (`self.Laser5`) (`self.Laser6`) (`self.Laser7`) (`self.Laser8`))))

(event `self.ReceiveTick`
  (params (DeltaSeconds :type "Float (single-precision)"))
  (if (and (<= (`KismetMathLibrary.RandomIntegerInRange` 1 100) 5) (not (`self.Wait`)))
    (set `self.Wait` true)
    (bind (_direction _float) (`Timeline|Shot` :!via `PlayFromStart`)
      (:`Update`
        (`SceneComponent.SetVisibility` (`|GetArrayItem` (`self.Lasers`) (`KismetMathLibrary.FTrunc` _float)) true false))
      (:`Finished`
        (`KismetSystemLibrary.Delay` 1.0)
        (`SceneComponent.SetVisibility` (`self.Center`) true false)
        (`KismetSystemLibrary.Delay` 3.0)
        (for _array_element (`self.Lasers`)
          (`SceneComponent.SetVisibility` _array_element false false))
        (`SceneComponent.SetVisibility` (`self.Center`) false false)
        (set `self.Wait` false)))))

(fn `UserConstructionScript`)