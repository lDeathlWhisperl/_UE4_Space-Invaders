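; Map component that spawns decorative background BP_EnemyLaser actors on random ticks, with randomized variants and an optional green material.
; The LaserMove timeline lerps the laser along the actor's forward vector to the Sphere's Distance-set X offset, then destroys it.
; Only one Laser reference is kept, so each spawn replaces it and restarts the timeline, leaving earlier lasers untracked.
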(event `self.ReceiveTick`
  (params (DeltaSeconds :type "Float (single-precision)"))
  (bind (_returnvalue_roll _returnvalue_pitch _returnvalue_yaw) (`KismetMathLibrary.BreakRotator` (`self.K2_GetActorRotation`)))
  ;[1 1 1] spawn laser
  (if (<= (`KismetMathLibrary.RandomIntegerInRange` 1 100) 60)
    (bind _returnvalue (`|SpawnActorFromClass` "/Game/Blueprints/Lasers/BP_EnemyLaser.BP_EnemyLaser_C" (`KismetMathLibrary.MakeTransform` (`self.K2_GetActorLocation`) (`KismetMathLibrary.MakeRotator` 90.0 _returnvalue_pitch _returnvalue_yaw)) "Undefined" "OverrideRootScale" null (`KismetMathLibrary.RandomBool`) (`KismetMathLibrary.RandomBool`) true null))
    (set `self.Laser` _returnvalue)
    (if (not (`KismetMathLibrary.RandomBool`))
      (`PrimitiveComponent.SetMaterial` (`/Game/Blueprints/Lasers/BP_EnemyLaser.Laser` (`self.Laser`)) 0 "/Game/Blueprints/Lasers/MAT_GreenLaser.MAT_GreenLaser")
      (`PrimitiveComponent.SetMaterial` (`/Game/Blueprints/Lasers/BP_EnemyLaser.ExtraLaser(instance)` (`self.Laser`)) 0 "/Game/Blueprints/Lasers/MAT_GreenLaser.MAT_GreenLaser"))
    (`TimelineComponent.PlayFromStart` (`self.LaserMove`))))

(fn `UserConstructionScript`
  (set `self.Type` (`self.Type`))
  (`SceneComponent.K2_SetRelativeLocation` (`self.Sphere`) (`KismetMathLibrary.MakeVector` (`self.Distance`)) false false))