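; BP_Spawner is an enemy wave spawner that refills the playing area once no actors tagged "Enemy" remain.
; A throttled Tick detects this, plays the WB_Trunsition animation, then spawns a row of enemies along Y from a construction-script mesh point, with a flyby sound.
; Spawners at a specific X set each enemy's Group flag.
; The random TIE-or-Alien roll can never select TIE, so it always sets Alien for subsequent spawns.
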(event `self.ReceiveBeginPlay`
  ;[1 1 1] HUD
  (bind _returnvalue (`|CreateWidget` "/Game/HUD/WB_Trunsition.WB_Trunsition_C"))
  (set `self.HUD` _returnvalue)
  (`UserWidget.AddToViewport` (`self.HUD`) 0))

(event `self.ReceiveTick`
  (params (DeltaSeconds :type "Float (single-precision)"))
  ;[1 1 1] Chekin' on empty playing area
  (`self.SetActorTickInterval` 5.0)
  (bind _outactors (`GameplayStatics.GetAllActorsWithTag` "Enemy"))
  (if (== (`KismetArrayLibrary.Array_Length` _outactors) 0)
    (`/Game/HUD/WB_Trunsition.Play_Anim` (`self.HUD`))
    (`KismetSystemLibrary.Delay` 2.0)
    (for _ (range 1 9)
      (`self.Spawn`)
      (if (<= (`KismetMathLibrary.RandomIntegerInRange` 1 100) 0)
        (set `self.Enemy` "/Game/Blueprints/Enemy/BP_TIE.BP_TIE_C")
        (else
          (set `self.Enemy` "/Game/Blueprints/Enemy/BP_Alien.BP_Alien_C"))))
    (set `self.Y` 0.0)
    (`GameplayStatics.PlaySoundAtLocation` "/Game/Sounds/SW_TIEFlyby.SW_TIEFlyby" (0.0 0.0 0.0) (struct) 1.0 1.0 0.0 null null null)))

(event `Spawn`
  (bind _returnvalue_x (`KismetMathLibrary.BreakVector` (`SceneComponent.K2_GetComponentLocation` (`self.SpawnPoint`))))
  (bind _returnvalue (== _returnvalue_x 1510.0))
  ;[1 1 1] Spawning
  (bind _returnvalue_2 (`|SpawnActorFromClass` (`self.Enemy`) (`KismetMathLibrary.MakeTransform` (+ (`SceneComponent.K2_GetComponentLocation` (`self.SpawnPoint`)) (`KismetMathLibrary.MakeVector` 0.0 (`self.Y`)))) "Undefined" "OverrideRootScale" null null))
  (set `self.Y` (+ 200.0 (`self.Y`)))
  (bind _asbp_tie (cast `/Game/Blueprints/Enemy/BP_TIE` _returnvalue_2)
    (:`then`
      (if _returnvalue
        (set `/Game/Blueprints/Enemy/BP_TIE.Group` true _asbp_tie)))
    (:`CastFailed`
      (bind _asbp_alien (cast `/Game/Blueprints/Enemy/BP_Alien` _returnvalue_2))
      (if _returnvalue
        (set `/Game/Blueprints/Enemy/BP_Alien.Group` true _asbp_alien)))))

(fn `UserConstructionScript`
  (bind _returnvalue (`AddComponent|NODE_AddStaticMeshComponent-0` :`RelativeTransform` (`KismetMathLibrary.MakeTransform` (0.0 0.0 0.0) (struct) (0.1 0.1 0.1))))
  (set `self.SpawnPoint` _returnvalue))