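; BP_DeathStar is a Death Star Blueprint with laser components aimed at a common center point.
; On BeginPlay it gathers the eight laser components into a Lasers array.
; TraceToCenter runs a Visibility line trace from a given component to Center, drawn as a timed green debug line.
; Nothing in the graphs calls TraceToCenter or reads the array, and the trace result is unused.
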(event `self.ReceiveBeginPlay`
  (set `self.Lasers` (`|MakeArray` (`self.Laser1`) (`self.Laser2`) (`self.Laser3`) (`self.Laser4`) (`self.Laser5`) (`self.Laser6`) (`self.Laser7`) (`self.Laser8`))))

(fn `TraceToCenter`
  (params (Component :type "StaticMeshComponent Object Reference"))
  (`KismetSystemLibrary.LineTraceSingle` :`Start` (`SceneComponent.K2_GetComponentLocation` Component) :`End` (`SceneComponent.K2_GetComponentLocation` (`self.Center`)) :`TraceChannel` "TraceTypeQuery1" :`DrawDebugType` "ForDuration" :`TraceColor` (struct :`G` 1.0 :`B` 0.005 :`A` 1.0)))

(fn `UserConstructionScript`)