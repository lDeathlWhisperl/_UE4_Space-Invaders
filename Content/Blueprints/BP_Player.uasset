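; Player ship Blueprint that moves left and right, fires twin lasers and creates the score HUD on BeginPlay.
; Fire spawns a laser at each gun with a volume-scaled sound, but only when neither previous laser still exists.
; The LaserMovements timeline lerps both lasers from their saved gun locations toward a fixed X, then destroys them.
; Tab or Escape opens the escape menu and pauses the game.
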(event `Key|Tab` :paused true
  (params (Key :type "Key Structure"))
  ;[1 1 1] Set game in pause
  (:`Pressed`
    (bind _returnvalue (`|CreateWidget` "/Game/HUD/WB_EscMenu.WB_EscMenu_C" :!label _label))
    (`UserWidget.AddToViewport` _returnvalue 0)
    (`WidgetBlueprintLibrary.SetInputMode_UIOnlyEx` (`GameplayStatics.GetPlayerController` 0) null)
    (`GameplayStatics.SetGamePaused` true)
    (set `PlayerController.bShowMouseCursor` true (`GameplayStatics.GetPlayerController` 0))))

(event `InputAxis|Move left/Right`
  (params (AxisValue :type "Float (single-precision)"))
  ;[1 1 1] Movements
  (`self.AddMovementInput` (`self.GetActorRightVector`) AxisValue))

(event `self.ReceiveBeginPlay`
  ;[1 1 1] Create HUD
  (bind _returnvalue (`|CreateWidget` "/Game/HUD/WB_Score.WB_Score_C"))
  (bind _output_get (set `self.HUD` _returnvalue))
  (`UserWidget.AddToViewport` _output_get 0)
  (bind _asgame_instance (cast `/Game/GameInstance` (`GameplayStatics.GetGameInstance`)))
  (set `self.GameInstance` _asgame_instance))

(event `Key|Escape` :paused true
  (params (Key :type "Key Structure"))
  ;[1 1 1] Set game in pause
  (:`Pressed`
    (goto _label)))

(event `InputAction|Fire`
  (params (Key :type "Key Structure"))
  ;[1 1 1] Shooting
  (:`Pressed`
    (if (not (or (`KismetSystemLibrary.IsValid` (`self.Right Laser`)) (`KismetSystemLibrary.IsValid` (`self.LeftLaser`))))
      (bind _laser (`self.Shoot` (`self.RightGun`)))
      (set `self.Right Laser` _laser)
      (bind _laser_2 (`self.Shoot` (`self.LeftGun`)))
      (set `self.LeftLaser` _laser_2)
      (`GameplayStatics.SpawnSoundAtLocation` "/Game/Sounds/SW_XWingFire.SW_XWingFire" (0.0 0.0 0.0) (struct) (/ (`KismetStringLibrary.Conv_StringToDouble` (`KismetTextLibrary.Conv_TextToString` (`/Game/GameInstance.EffectsVolume` (`self.GameInstance`)))) 100.0) 1.0 0.0 null null)
      (set `self.LeftGunLocation` (`SceneComponent.K2_GetComponentLocation` (`self.LeftGun`)))
      (set `self.RightGunLocation` (`SceneComponent.K2_GetComponentLocation` (`self.RightGun`)))
      (`TimelineComponent.PlayFromStart` (`self.LaserMovements`)))))

(fn `SetLaserLocation`
  (params (Laser :type "/Game/Blueprints/Lasers/BP_PlayerLaser Object Reference") (GunLocation :type "Vector Structure") (Alpha :type "Float (double-precision)"))
  (`self.K2_SetActorLocation` Laser (`KismetMathLibrary.VLerp` GunLocation (`KismetMathLibrary.MakeVector` 800.0 (.y GunLocation)) Alpha) false false))

(fn `Shoot`
  (params (Gun :type "StaticMeshComponent Object Reference"))
  (returns (Laser :type "/Game/Blueprints/Lasers/BP_PlayerLaser Object Reference"))
  (bind _returnvalue (`|SpawnActorFromClass` "/Game/Blueprints/Lasers/BP_PlayerLaser.BP_PlayerLaser_C" (`KismetMathLibrary.MakeTransform` (+ (`SceneComponent.K2_GetComponentLocation` Gun) (20.0 0.0 0.0))) "Undefined" "OverrideRootScale" null null))
  (return _returnvalue))

(fn `UserConstructionScript`)