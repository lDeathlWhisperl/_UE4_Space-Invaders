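; BP_ClassicAlien is an enemy alien that fires lasers and dies when its Box overlaps a player laser.
; Tick gates shooting with a two-second reload, rolling a roughly 40% chance to spawn a BP_EnemyLaser at the Gun.
; The alien itself moves its latest laser along negative X by a fixed per-frame offset, not scaled by delta time.
; On death it destroys itself, the player laser and that tracked laser.
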(event `self.Box.OnComponentBeginOverlap`
  (params (OverlappedComponent :type "PrimitiveComponent Object Reference") (OtherActor :type "Actor Object Reference") (OtherComp :type "PrimitiveComponent Object Reference") (OtherBodyIndex :type Integer) (bFromSweep :type Boolean) (SweepResult :type "HitResult Structure (by ref)"))
  (bind _laser (`self.Laser`))
  ;[1 1 1] Death
  (bind _asbp_player_laser (cast `/Game/Blueprints/Lasers/BP_PlayerLaser` OtherActor))
  (`self.K2_DestroyActor`)
  (`self.K2_DestroyActor` _asbp_player_laser)
  (`/Engine/EditorBlueprintResources/StandardMacros.IsValid` _laser
    (:`Is Valid`
      (`self.K2_DestroyActor` _laser))))

(event `self.ReceiveTick`
  (params (DeltaSeconds :type "Float (single-precision)"))
  ;[1 1 1] Shooting system
  (`self.Laser Movement`)
  (if (not (`self.IsReloading`))
    (set `self.CanShoot` (<= (`KismetMathLibrary.RandomInteger` 100) 40))
    (set `self.IsReloading` true)
    (`self.Shoot`)
    (`KismetSystemLibrary.Delay` 2.0)
    (set `self.IsReloading` false)))

(event `Shoot`
  ;[1 1 1] Shooting system
  (if (`self.CanShoot`)
    (bind _laser (`self.SpawnLaser` (`self.Gun`)))
    (set `self.Laser` _laser)))

(event `Laser Movement`
  ;[1 1 1] Shooting system
  (`/Engine/EditorBlueprintResources/StandardMacros.IsValid` (`self.Laser`)
    (:`Is Valid`
      (`self.K2_AddActorWorldOffset` (`self.Laser`) (-15.0 0.0 0.0) false false))))

(fn `SpawnLaser`
  (params (Gun :type "StaticMeshComponent Object Reference"))
  (returns (Laser :type "/Game/Blueprints/Lasers/BP_EnemyLaser Object Reference"))
  (bind _returnvalue (`|SpawnActorFromClass` "/Game/Blueprints/Lasers/BP_EnemyLaser.BP_EnemyLaser_C" (`KismetMathLibrary.MakeTransform` (- (`SceneComponent.K2_GetComponentLocation` Gun) (20.0 0.0 0.0))) "Undefined" "OverrideRootScale" null null))
  (return _returnvalue))

(fn `UserConstructionScript`)