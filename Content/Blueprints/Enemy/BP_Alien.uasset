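; BP_Alien is an enemy that flies from its spawn point into the playable area, then strafes left or right based on Group.
; Timelines drive the movement, starting from the construction script.
; Shooting logic rolls a roughly 40% chance to fire BP_EnemyLaser, with a two-second reload and a brief cube-reshaping animation.
; Death spawns an 8-bit explosion and destroys the actor, with sound effects scaled by GameInstance volume.
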(event `self.ReceiveBeginPlay`
  (bind _asgame_instance (cast `/Game/GameInstance` (`GameplayStatics.GetGameInstance`)))
  (set `self.GameInstance` _asgame_instance))

(event `Death`
  ;[1 1 1] Death
  (bind _value (`self.GetVolumeLevel` (`self.GameInstance`)))
  (`GameplayStatics.PlaySoundAtLocation` "/Game/Sounds/SW_8BitExplosion.SW_8BitExplosion" (0.0 0.0 0.0) (struct) _value 1.0 0.0 null null null)
  (`GameplayStatics.SpawnEmitterAtLocation` "/Game/Particles/P_8BitExplosion.P_8BitExplosion" (`self.K2_GetActorLocation`))
  (`self.K2_DestroyActor`))

(event `When spawned`
  ;[1 1 1] When spawned move to playable area
  (bind (_direction _float) (`Timeline|Move to`)
    (:`Update`
      (`self.K2_SetActorLocation` (`KismetMathLibrary.VLerp` (`self.StartLocation`) (`self.EndLocation`) _float))
      (set `self.StrafeRight` (+ (`self.EndLocation`) (0.0 100.0 0.0)))
      (set `self.StrafeLeft` (- (`self.EndLocation`) (0.0 100.0 0.0)))
      (`self.Strafe`))))

(event `self.ReceiveTick`
  (params (DeltaSeconds :type "Float (single-precision)"))
  ;[1 1 1] Shooting system
  (`|ExecutionSequence`
    (:`then_0`
      (if (`self.WasRecentlyRendered` 0.2)
        (if (not (`self.IsReloading`))
          (set `self.CanShoot` (<= (`KismetMathLibrary.RandomIntegerInRange` 0 100) 40))
          (set `self.IsReloading` true)
          (`self.Shoot`)
          (`KismetSystemLibrary.Delay` 2.0)
          (set `self.IsReloading` false))))))

(event `Strafe`
  ;[1 1 1] Strafe
  (`KismetSystemLibrary.Delay` 3.0)
  (bind (_direction _float) (`Timeline|Left/Right`)
    (:`Update`
      (if (`self.Group`)
        (`self.K2_SetActorLocation` (`KismetMathLibrary.VLerp` (`self.EndLocation`) (`self.StrafeRight`) _float))
        (else
          (`self.K2_SetActorLocation` (`KismetMathLibrary.VLerp` (`self.EndLocation`) (`self.StrafeLeft`) _float)))))))

(event `Shoot`
  ;[1 1 1] Shooting system
  (if (`self.CanShoot`)
    (`self.Animation`)
    (`self.SpawnLaser` (`self.Gun`))
    (bind _value (`self.GetVolumeLevel` (`self.GameInstance`)))
    (`GameplayStatics.PlaySoundAtLocation` "/Game/Sounds/SW_8BitLaser.SW_8BitLaser" (0.0 0.0 0.0) (struct) _value 1.0 0.0 null null null)))

(event `Animation`
  ;[1 1 1] Alien Animation
  (`|ExecutionSequence`
    (:`then_0`
      (`SceneComponent.SetRelativeScale3D` (`self.Cube`) (0.1 0.9 0.00625)))
    (:`then_1`
      (`SceneComponent.K2_SetRelativeLocation` (`self.Cube3`) (-20.0 -40.0 0.0) false false)
      (`SceneComponent.SetRelativeScale3D` (`self.Cube3`) (0.1 0.1 0.00625)))
    (:`then_2`
      (`SceneComponent.K2_SetRelativeLocation` (`self.Cube4`) (-20.0 40.0 0.0) false false)
      (`SceneComponent.SetRelativeScale3D` (`self.Cube4`) (0.1 0.1 0.00625)))
    (:`then_3`
      (`SceneComponent.K2_SetRelativeLocation` (`self.Cube5`) (25.0 -50.0 0.0) false false))
    (:`then_4`
      (`SceneComponent.K2_SetRelativeLocation` (`self.Cube6`) (25.0 50.0 0.0) false false)
      (`KismetSystemLibrary.Delay` 0.5)
      (`|ExecutionSequence`
        (:`then_0`
          (`SceneComponent.SetRelativeScale3D` (`self.Cube`) (0.1 0.7 0.00625)))
        (:`then_1`
          (`SceneComponent.K2_SetRelativeLocation` (`self.Cube3`) (-20.0 -15.0 0.0) false false)
          (`SceneComponent.SetRelativeScale3D` (`self.Cube3`) (0.1 0.2 0.00625)))
        (:`then_2`
          (`SceneComponent.K2_SetRelativeLocation` (`self.Cube4`) (-20.0 15.0 0.0) false false)
          (`SceneComponent.SetRelativeScale3D` (`self.Cube4`) (0.1 0.2 0.00625)))
        (:`then_3`
          (`SceneComponent.K2_SetRelativeLocation` (`self.Cube5`) (-5.0 -50.0 0.0) false false))
        (:`then_4`
          (`SceneComponent.K2_SetRelativeLocation` (`self.Cube6`) (-5.0 50.0 0.0) false false))))))

(fn `GetVolumeLevel`
  (params (Target :type "/Game/GameInstance Object Reference"))
  (returns (Value :type "Float (double-precision)"))
  (return (/ (`KismetStringLibrary.Conv_StringToDouble` (`KismetTextLibrary.Conv_TextToString` (`/Game/GameInstance.EffectsVolume` Target))) 100.0)))

(fn `SpawnLaser`
  (params (Gun :type "StaticMeshComponent Object Reference"))
  (`|SpawnActorFromClass` "/Game/Blueprints/Lasers/BP_EnemyLaser.BP_EnemyLaser_C" (`KismetMathLibrary.MakeTransform` (- (`SceneComponent.K2_GetComponentLocation` Gun) (20.0 0.0 0.0))) "Undefined" "OverrideRootScale" null false false null))

(fn `UserConstructionScript`
  (bind _output_get (set `self.StartLocation` (`self.K2_GetActorLocation`)))
  (set `self.EndLocation` (- _output_get (1160.0 0.0 500.0)))
  (`self.When spawned`))