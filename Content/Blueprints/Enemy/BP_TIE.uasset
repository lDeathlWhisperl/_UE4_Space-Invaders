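; BP_TIE is a TIE enemy that is destroyed, along with its live lasers, when a player laser overlaps its Box.
; Shoot spawns a BP_EnemyLaser at each of two guns, keeping references that LaserMovements uses to slide them along negative X.
; The chain that calls both, with a random fire chance and reload delay, is disconnected from the empty Tick, so it never runs.
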(event `self.Box.OnComponentBeginOverlap`
  (params (OverlappedComponent :type "PrimitiveComponent Object Reference") (OtherActor :type "Actor Object Reference") (OtherComp :type "PrimitiveComponent Object Reference") (OtherBodyIndex :type Integer) (bFromSweep :type Boolean) (SweepResult :type "HitResult Structure (by ref)"))
  ;[1 1 1] Death
  (bind _asbp_player_laser (cast `/Game/Blueprints/Lasers/BP_PlayerLaser` OtherActor))
  (`self.K2_DestroyActor`)
  (`self.K2_DestroyActor` _asbp_player_laser)
  (`/Engine/EditorBlueprintResources/StandardMacros.IsValid` (`self.RightLaser`)
    (:`Is Valid`
      (`self.K2_DestroyActor` (`self.RightLaser`))
      (`/Engine/EditorBlueprintResources/StandardMacros.IsValid` (`self.LeftLaser`)
        (:`Is Valid`
          (`self.K2_DestroyActor` (`self.LeftLaser`)))))))

(event `self.ReceiveTick`
  (params (DeltaSeconds :type "Float (single-precision)"))
  ;[1 1 1] Shooting System
)

(event `Shoot`
  ;[1 1 1] Shooting System
  (if (`self.CanShoot`)
    (bind _laser (`self.SpawnLaser` (`self.Right Gun`)))
    (set `self.RightLaser` _laser)
    (bind _laser_2 (`self.SpawnLaser` (`self.Left Gun`)))
    (set `self.LeftLaser` _laser_2)))

(event `Laser Movements`
  ;[1 1 1] Shooting System
  (`|ExecutionSequence`
    (:`then_0`
      (`/Engine/EditorBlueprintResources/StandardMacros.IsValid` (`self.RightLaser`)
        (:`Is Valid`
          (`self.K2_AddActorWorldOffset` (`self.RightLaser`) (-15.0 0.0 0.0) false false))))
    (:`then_1`
      (`/Engine/EditorBlueprintResources/StandardMacros.IsValid` (`self.LeftLaser`)
        (:`Is Valid`
          (`self.K2_AddActorWorldOffset` (`self.LeftLaser`) (-15.0 0.0 0.0) false false))))))

(fn `SpawnLaser`
  (params (Gun :type "StaticMeshComponent Object Reference"))
  (returns (Laser :type "/Game/Blueprints/Lasers/BP_EnemyLaser Object Reference"))
  (bind _returnvalue (`|SpawnActorFromClass` "/Game/Blueprints/Lasers/BP_EnemyLaser.BP_EnemyLaser_C" (`KismetMathLibrary.MakeTransform` (- (`SceneComponent.K2_GetComponentLocation` Gun) (20.0 0.0 0.0))) "Undefined" "OverrideRootScale" null null))
  (return _returnvalue))

(fn `UserConstructionScript`)