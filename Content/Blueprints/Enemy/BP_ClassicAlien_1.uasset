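; Classic alien enemy for a shooter that destroys itself and its active laser when hit by a player laser.
; The construction script sets the path and starts a timeline lerp into the play area, followed by a delayed left or right strafe chosen by Group.
; Tick runs a delay-gated random shot, moves the latest spawned laser itself, and animates the cube body by toggling part transforms.
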(event `self.Box.OnComponentBeginOverlap`
  (params (OverlappedComponent :type "PrimitiveComponent Object Reference") (OtherActor :type "Actor Object Reference") (OtherComp :type "PrimitiveComponent Object Reference") (OtherBodyIndex :type Integer) (bFromSweep :type Boolean) (SweepResult :type "HitResult Structure (by ref)"))
  (bind _laser (`self.Laser`))
  ;[1 1 1] Death
  (bind _asbp_player_laser (cast `/Game/Blueprints/Lasers/BP_PlayerLaser` OtherActor))
  (`self.K2_DestroyActor`)
  (`self.K2_DestroyActor` _asbp_player_laser)
  (`/Engine/EditorBlueprintResources/StandardMacros.IsValid` _laser
    (:`Is Valid`
      (`self.K2_DestroyActor` _laser))))

(event `When spawned`
  ;[1 1 1] When spawned move to playable area
  (bind (_direction _float) (`Timeline|Timeline_0`)
    (:`Update`
      (`self.K2_SetActorLocation` (`KismetMathLibrary.VLerp` (`self.StartLocation`) (`self.EndLocation`) _float))
      (set `self.StrafeRight` (+ (`self.EndLocation`) (0.0 100.0 0.0)))
      (set `self.StrafeLeft` (- (`self.EndLocation`) (0.0 100.0 0.0)))
      (`self.Strafe`))))

(event `Strafe`
  ;[1 1 1] Strafe
  (`KismetSystemLibrary.Delay` 3.0)
  (bind (_direction _float) (`Timeline|Timeline_1`)
    (:`Update`
      (if (`self.Group`)
        (`self.K2_SetActorLocation` (`KismetMathLibrary.VLerp` (`self.EndLocation`) (`self.StrafeRight`) _float))
        (else
          (`self.K2_SetActorLocation` (`KismetMathLibrary.VLerp` (`self.EndLocation`) (`self.StrafeLeft`) _float)))))))

(event `Shoot`
  ;[1 1 1] Shooting system
  (if (`self.CanShoot`)
    (bind _laser (`self.SpawnLaser` (`self.Gun`)))
    (set `self.Laser` _laser)))

(event `self.ReceiveTick`
  (params (DeltaSeconds :type "Float (single-precision)"))
  (`|ExecutionSequence`
    (:`then_0`
      ;[1 1 1] Shooting system
      (`self.Laser Movement`)
      (if (not (`self.IsReloading`))
        (set `self.CanShoot` (<= (`KismetMathLibrary.RandomInteger` 100) 40))
        (set `self.IsReloading` true)
        (`self.Shoot`)
        (`KismetSystemLibrary.Delay` 2.0)
        (set `self.IsReloading` false)))
    (:`then_1`
      (`self.Animation`))))

(event `Laser Movement`
  ;[1 1 1] Shooting system
  (`/Engine/EditorBlueprintResources/StandardMacros.IsValid` (`self.Laser`)
    (:`Is Valid`
      (`self.K2_AddActorWorldOffset` (`self.Laser`) (-15.0 0.0 0.0) false false))))

(event `Animation`
  ;[1 1 1] Alien Animation
  (`KismetSystemLibrary.Delay` 1.0)
  (`|ExecutionSequence`
    (:`then_0`
      (`SceneComponent.SetRelativeScale3D` (`self.Cube`) (0.1 0.9 0.00625)))
    (:`then_1`
      (`SceneComponent.K2_SetRelativeLocation` (`self.Cube3`) (-20.0 -40.0 0.0) false false)
      (`SceneComponent.SetRelativeScale3D` (`self.Cube3`) (0.1 0.1 0.00625))
      (`KismetSystemLibrary.Delay` 1.5)
      (`|ExecutionSequence`
        (:`then_0`
          (`SceneComponent.SetRelativeScale3D` (`self.Cube`) (0.1 0.7 0.00625)))
        (:`then_1`
          (`SceneComponent.K2_SetRelativeLocation` (`self.Cube3`) (-20.0 -15.0 0.0) false false)
          (`SceneComponent.SetRelativeScale3D` (`self.Cube3`) (0.1 0.2 0.00625)))
        (:`then_2`
          (`SceneComponent.K2_SetRelativeLocation` (`self.Cube4`) (-20.0 15.0 0.0) false false)
          (`SceneComponent.SetRelativeScale3D` (`self.Cube4`) (0.1 0.2 0.00625)))
        (:`then_3`
          (`SceneComponent.K2_SetRelativeLocation` (`self.Cube5`) (-5.0 -50.0 0.0) false false))
        (:`then_4`
          (`SceneComponent.K2_SetRelativeLocation` (`self.Cube6`) (-5.0 50.0 0.0) false false))))
    (:`then_2`
      (`SceneComponent.K2_SetRelativeLocation` (`self.Cube4`) (-20.0 40.0 0.0) false false)
      (`SceneComponent.SetRelativeScale3D` (`self.Cube4`) (0.1 0.1 0.00625)))
    (:`then_3`
      (`SceneComponent.K2_SetRelativeLocation` (`self.Cube5`) (25.0 -50.0 0.0) false false))
    (:`then_4`
      (`SceneComponent.K2_SetRelativeLocation` (`self.Cube6`) (25.0 50.0 0.0) false false))))

(fn `SpawnLaser`
  (params (Gun :type "StaticMeshComponent Object Reference"))
  (returns (Laser :type "/Game/Blueprints/Lasers/BP_EnemyLaser Object Reference"))
  (bind _returnvalue (`|SpawnActorFromClass` "/Game/Blueprints/Lasers/BP_EnemyLaser.BP_EnemyLaser_C" (`KismetMathLibrary.MakeTransform` (- (`SceneComponent.K2_GetComponentLocation` Gun) (20.0 0.0 0.0))) "Undefined" "OverrideRootScale" null null))
  (return _returnvalue))

(fn `UserConstructionScript`
  (bind _output_get (set `self.StartLocation` (`self.K2_GetActorLocation`)))
  (set `self.EndLocation` (- _output_get (1160.0 0.0 500.0)))
  (`self.When spawned`))