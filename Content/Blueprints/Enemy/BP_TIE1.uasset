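; TIE fighter enemy that builds a formation of instanced ships, guns and DeathRoll components from Row and Line counts.
; A timeline flies it from spawn into the play area, then another strafes it sideways by Group.
; Tick drives timed, random-chance twin laser shots and moves the latest pair itself.
; DeathAnim activates fire, then explodes and destroys the actor, but its player-laser hit trigger is unwired.
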(event `Death Anim`
  ;[1 1 1] Death Animatuon
  (set `self.IsDying` true)
  (`ActorComponent.Activate` (`self.Fire`) false)
  (`KismetSystemLibrary.Delay` 3.0)
  (`GameplayStatics.SpawnEmitterAtLocation` "/Game/StarterContent/Particles/P_Explosion.P_Explosion" (`self.K2_GetActorLocation`))
  (`self.K2_DestroyActor`))

(event `When spawned`
  ;[1 1 1] When spawned move to playable area
  (bind (_direction _float) (`Timeline|Move to`)
    (:`Update`
      (`self.K2_SetActorLocation` (`KismetMathLibrary.VLerp` (`self.StartLocation`) (`self.EndLocation`) _float))
      (set `self.StrafeRight` (+ (`self.EndLocation`) (0.0 100.0 0.0)))
      (set `self.StrafeLeft` (- (`self.EndLocation`) (0.0 100.0 0.0)))
      (`self.Strafe`))))

(event `self.ReceiveTick`
  (params (DeltaSeconds :type "Float (single-precision)"))
  ;[1 1 1] Shooting System
  (`self.Laser Movements`)
  (if (not (or (`self.IsReloading`) (`self.IsDying`)))
    (set `self.CanShoot` (<= (`KismetMathLibrary.RandomInteger` 100) 40))
    (set `self.IsReloading` true)
    (`self.Shoot`)
    (`KismetSystemLibrary.Delay` 2.0)
    (set `self.IsReloading` false)))

(event `Shoot`
  ;[1 1 1] Shooting System
  (if (`self.CanShoot`)
    (bind _laser (`self.SpawnLaser` (`self.RightGun`)))
    (set `self.RightLaser` _laser)
    (bind _laser_2 (`self.SpawnLaser` (`self.LeftGun`)))
    (set `self.LeftLaser` _laser_2)))

(event `Laser Movements`
  ;[1 1 1] Shooting System
  (`|ExecutionSequence`
    (:`then_0`
      (`/Engine/EditorBlueprintResources/StandardMacros.IsValid` (`self.RightLaser`)
        (:`Is Valid`
          (`self.K2_AddActorWorldOffset` (`self.RightLaser`) (-15.0 0.0 0.0) false false))))
    (:`then_1`
      (`/Engine/EditorBlueprintResources/StandardMacros.IsValid` (`self.LeftLaser`)
        (:`Is Valid`
          (`self.K2_AddActorWorldOffset` (`self.LeftLaser`) (-15.0 0.0 0.0) false false))))))

(event `Strafe`
  ;[1 1 1] Strafe
  (if (not (`self.IsDying`))
    (`KismetSystemLibrary.Delay` 3.0)
    (bind (_direction _float) (`Timeline|Left/Right`)
      (:`Update`
        (if (`self.Group`)
          (`self.K2_SetActorLocation` (`KismetMathLibrary.VLerp` (`self.EndLocation`) (`self.StrafeRight`) _float))
          (else
            (`self.K2_SetActorLocation` (`KismetMathLibrary.VLerp` (`self.EndLocation`) (`self.StrafeLeft`) _float))))))))

(fn `SpawnLaser`
  (params (Gun :type "StaticMeshComponent Object Reference"))
  (returns (Laser :type "/Game/Blueprints/Lasers/BP_EnemyLaser Object Reference"))
  (bind _returnvalue (`|SpawnActorFromClass` "/Game/Blueprints/Lasers/BP_EnemyLaser.BP_EnemyLaser_C" (`KismetMathLibrary.MakeTransform` (- (`SceneComponent.K2_GetComponentLocation` Gun) (20.0 0.0 0.0))) "Undefined" "OverrideRootScale" null null))
  (return _returnvalue))

(fn `UserConstructionScript`
  (locals (X :type "Float (double-precision)") (NewLocalVar_0 :type Integer) (NewLocalVar_1 :type Integer))
  (`|ExecutionSequence`
    (:`then_0`
      (bind _output_get (set `self.StartLocation` (`self.K2_GetActorLocation`)))
      (set `self.EndLocation` (- _output_get (1160.0 0.0 500.0)))
      (`self.When spawned`))
    (:`then_1`
      (for _ (range 1 (+ (`self.Row`) 1))
        (for _index (range (`self.Line`))
          (bind _returnvalue (* _index 200.0))
          (`InstancedStaticMeshComponent.AddInstance` (`self.TIE`) (`KismetMathLibrary.MakeTransform` (`KismetMathLibrary.MakeVector` (`local.X`) _returnvalue) (struct :`Yaw` 90.0) (0.15 0.15 0.15)))
          (`InstancedStaticMeshComponent.AddInstance` (`self.LeftGun`) (`KismetMathLibrary.MakeTransform` (`KismetMathLibrary.MakeVector` (`local.X`) _returnvalue) (struct) (0.01 0.01 0.01)))
          (`InstancedStaticMeshComponent.AddInstance` (`self.RightGun`) (`KismetMathLibrary.MakeTransform` (`KismetMathLibrary.MakeVector` (`local.X`) _returnvalue) (struct) (0.01 0.01 0.01)))
          (`InstancedStaticMeshComponent.AddInstance` (`self.DeathRoll`) (`KismetMathLibrary.MakeTransform` (`KismetMathLibrary.MakeVector` (`local.X`) _returnvalue) (struct) (0.1 0.1 0.1)))
          (if (== 2 (`self.Row`))
            (set `self.Group` false)))
        (set `local.X` (- (`local.X`) -170.0))))))